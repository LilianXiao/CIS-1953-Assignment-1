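; BP_MovingTarget is a spinning prism target that jumps to a random location when something overlaps it.
; Any overlap on the Prism calls TeleportWithinRange, which picks X and Y between RangeMin and RangeMax and Z from a fixed height band, in absolute world coordinates.
; Tick adds a fixed rotation each frame, so spin speed depends on frame rate.
; The BP_Projectile cast is unconnected, and the saved StartingPlace is never read.
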(event `self.ReceiveBeginPlay`
  (set `self.StartingPlace` (`KismetMathLibrary.MakeTransform` (`self.K2_GetActorLocation`) (`self.K2_GetActorRotation`))))

(event `self.Prism.OnComponentBeginOverlap`
  (params (OverlappedComponent :type "PrimitiveComponent Object Reference") (OtherActor :type "Actor Object Reference") (OtherComp :type "PrimitiveComponent Object Reference") (OtherBodyIndex :type Integer) (bFromSweep :type Boolean) (SweepResult :type "HitResult Structure (by ref)"))
  ; teleport trigger
  (`self.TeleportWithinRange`))

(event `self.ReceiveTick`
  (params (DeltaSeconds :type "Float (single-precision)"))
  ; prism rotation
  (`self.K2_SetActorRotation` self (`KismetMathLibrary.ComposeRotators` (`self.K2_GetActorRotation` self) (struct :`Yaw` 3.0)) false))

(fn `TeleportWithinRange`
  (bind _rangemin (`self.RangeMin`))
  (bind _rangemax (`self.RangeMax`))
  (`self.K2_SetActorLocation` (`KismetMathLibrary.MakeVector` (`KismetMathLibrary.RandomFloatInRange` _rangemin _rangemax) (`KismetMathLibrary.RandomFloatInRange` _rangemin _rangemax) (`KismetMathLibrary.RandomFloatInRange` 200.0 400.0)) false true))

(fn `UserConstructionScript`)